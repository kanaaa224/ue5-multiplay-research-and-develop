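; Multiplayer main game mode that tracks player count against the game instance's MaxPlayers and handles travel back to the matching room.
; On login it kicks player controller 0 if over the limit, or loads saved state and flags everyone logged in when full.
; Later logouts shrink MaxPlayers, while OpenNextLevel saves state and runs servertravel to Level_MatchingRoom.
; PlayerDied restarts the player, but its binding never runs.
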(event `self.ReceiveBeginPlay`)

(event `PlayerDied` :!signature `self.OnPlayerDied`
  (params (Character :type "Character Object Reference"))
  (`self.RestartPlayer` (`Pawn.GetController` Character)))

(event `self.K2_PostLogin`
  (params (NewPlayer :type "PlayerController Object Reference"))
  (`|ExecutionSequence`
    (:`then_0`
      (bind _asgame_instance_main (cast `/Game/Multiplay/System/Blueprints/GameInstance_Main` (`GameplayStatics.GetGameInstance`)))
      (bind _players (`self.GetCurrentPlayers`))
      (if (> _players (`/Game/Multiplay/System/Blueprints/GameInstance_Main.MaxPlayers` _asgame_instance_main))
        (bind _asplayer_controller_main (cast `/Game/Multiplay/System/Blueprints/PlayerController_Main` (`GameplayStatics.GetPlayerController` 0)))
        (`/Game/Multiplay/System/Blueprints/PlayerController_Main.Kick` _asplayer_controller_main)))
    (:`then_1`
      (bind _asgame_instance_main_2 (cast `/Game/Multiplay/System/Blueprints/GameInstance_Main` (`GameplayStatics.GetGameInstance`)))
      (bind _players_2 (`self.GetCurrentPlayers`))
      (if (== _players_2 (`/Game/Multiplay/System/Blueprints/GameInstance_Main.MaxPlayers` _asgame_instance_main_2))
        (`/Game/Multiplay/System/Blueprints/GameInstance_Main.LoadGameState` _asgame_instance_main_2)
        (set `self.isAllPlayerLoggedIn` true)
        (bind _asgame_state_main (cast `/Game/Multiplay/System/Blueprints/GameState_Main` (`GameplayStatics.GetGameState`)))
        (set `/Game/Multiplay/System/Blueprints/GameState_Main.isAllPlayerLoggedIn` true _asgame_state_main)))))

(event `self.K2_OnLogout`
  (params (ExitingController :type "Controller Object Reference"))
  (if (`self.isAllPlayerLoggedIn`)
    (bind _asgame_instance_main (cast `/Game/Multiplay/System/Blueprints/GameInstance_Main` (`GameplayStatics.GetGameInstance`)))
    (bind _players (`self.GetCurrentPlayers`))
    (bind _result (`/Engine/EditorBlueprintResources/StandardMacros.DecrementInt` _players)
      (:`  `
        (set `/Game/Multiplay/System/Blueprints/GameInstance_Main.MaxPlayers` _result _asgame_instance_main)))))

(event `OpenNextLevel`
  (set `self.isAllPlayerLoggedIn` false)
  (bind _asgame_instance_main (cast `/Game/Multiplay/System/Blueprints/GameInstance_Main` (`GameplayStatics.GetGameInstance`)))
  (`/Game/Multiplay/System/Blueprints/GameInstance_Main.SaveGameState` _asgame_instance_main)
  (`KismetSystemLibrary.ExecuteConsoleCommand` (`KismetStringLibrary.Concat_StrStr` "servertravel " "/Game/UI/Maps/Level_MatchingRoom") (`GameplayStatics.GetPlayerController` 0)))

(fn `GetCurrentPlayers`
  (returns (Players :type Integer))
  (bind _asgame_state_main (cast `/Game/Multiplay/System/Blueprints/GameState_Main` (`GameplayStatics.GetGameState`)))
  (for (_ _array_index) (`GameStateBase.PlayerArray` _asgame_state_main)
    _)
  (return (+ _array_index 1)))

(fn `UserConstructionScript`)