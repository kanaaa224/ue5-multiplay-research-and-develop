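; Game instance Blueprint for multiplayer that wraps level travel in a loading screen.
; OpenLevel begins the loading screen, stream-loads the level hidden and non-blocking, opens it by name, then ends the screen.
; The screen is held by a loading process task created with a reason and later unregistered and cleared.
; As wired, Begin creates that task only if the stored one is already valid.
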(event `OpenLevel`
  (params (LoadingReason :type String) (LevelName :type Name))
  (`self.BeginLoadingScreen` LoadingReason)
  (`GameplayStatics.LoadStreamLevel` LevelName)
  (`GameplayStatics.OpenLevel` LevelName)
  (`self.EndLoadingScreen`))

(event `BeginLoadingScreen`
  (params (LoadingReason :type String))
  (`/Engine/EditorBlueprintResources/StandardMacros.IsValid` (`self.LoadingProcessTask`)
    (:`Is Valid`
      (bind _returnvalue (`LoadingProcessTask.CreateLoadingScreenProcessTask` LoadingReason))
      (set `self.LoadingProcessTask` _returnvalue))))

(event `EndLoadingScreen`
  (bind _loadingprocesstask (`self.LoadingProcessTask`)
    (:`then`
      (`LoadingProcessTask.Unregister` _loadingprocesstask)
      (set `self.LoadingProcessTask` null))
    (:`else`)))