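; Multiplayer player controller that shows the menu matching the current game mode, title or waiting room.
; On BeginPlay it creates both widgets, then casts the game mode to decide which one to add to the viewport, along with showing the mouse cursor.
; A Kick event sends the player back to the title level.
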(event `self.ReceiveBeginPlay`
  (bind _returnvalue (`GameplayStatics.GetGameMode`))
  (`|ExecutionSequence`
    (:`then_0`
      (bind _returnvalue_2 (`|CreateWidget` "/Game/Multiplay/Blueprints/widget_title.widget_title_C" self))
      (`Widget.RemoveFromParent` _returnvalue_2)
      (cast `/Game/Multiplay/Blueprints/GameMode-Title` _returnvalue)
      (`UserWidget.AddToViewport` _returnvalue_2 0)
      (set `self.bShowMouseCursor` true))
    (:`then_1`
      (bind _returnvalue_3 (`|CreateWidget` "/Game/Multiplay/Blueprints/widget_waitingRoom.widget_waitingRoom_C" self))
      (`Widget.RemoveFromParent` _returnvalue_3)
      (cast `/Game/Multiplay/Blueprints/GameMode-WaitingRoom` _returnvalue)
      (`UserWidget.AddToViewport` _returnvalue_3 0)
      (set `self.bShowMouseCursor` true))))

(event `Kick`
  (`GameplayStatics.OpenLevel` "title"))

(fn `UserConstructionScript`)