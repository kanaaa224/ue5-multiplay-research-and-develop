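; HUD class for the multiplayer waiting room that puts the waiting-room UI on the owning player's screen.
; On BeginPlay it creates the Widget_WaitingRoom widget, adds it to the viewport, then switches to Game and UI input focused on it with the mouse cursor shown.
; When destroyed, it restores Game Only input but does not hide the cursor or remove the widget.
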(event `self.ReceiveBeginPlay`
  (bind _returnvalue (`self.GetOwningPlayerController`))
  (`|ExecutionSequence`
    (:`then_0`
      ;[1 1 1] Widgetを作成してViewportに追加
      (bind _returnvalue_2 (`|CreateWidget` "/Game/Multiplay/Blueprints/Widget_WaitingRoom.Widget_WaitingRoom_C" _returnvalue))
      (bind _output_get (set `self.widgetRef` _returnvalue_2))
      (`UserWidget.AddToViewport` _output_get 0))
    (:`then_1`
      ;[1 1 1] マウスカーソルを表示
      (`WidgetBlueprintLibrary.SetInputMode_GameAndUIEx` _returnvalue (`self.widgetRef`))
      (set `PlayerController.bShowMouseCursor` true _returnvalue))))

(event `self.ReceiveDestroyed`
  (`WidgetBlueprintLibrary.SetInputMode_GameOnly` (`self.GetOwningPlayerController`)))

(fn `UserConstructionScript`)