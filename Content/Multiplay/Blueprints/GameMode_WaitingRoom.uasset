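; Waiting room game mode that enforces the multiplayer player cap when someone logs in.
; On PostLogin it compares the current player count against MaxPlayers from GameInstance_1.
; If the count exceeds the cap, it calls Kick on the PlayerController_1 at the last player index, rather than using the joining controller.
; GetCurrentPlayers derives the count from the last loop index over the GameState_1 PlayerArray.
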(event `self.ReceiveBeginPlay`)

(event `self.K2_PostLogin`
  (params (NewPlayer :type "PlayerController Object Reference"))
  (bind _asgame_instance_1 (cast `/Game/Multiplay/Blueprints/GameInstance_1` (`GameplayStatics.GetGameInstance`)))
  (bind _players (`self.GetCurrentPlayers`))
  (if (> _players (`/Game/Multiplay/Blueprints/GameInstance_1.maxPlayers` _asgame_instance_1))
    (bind _asplayer_controller_1 (cast `/Game/Multiplay/Blueprints/PlayerController_1` (`GameplayStatics.GetPlayerController` (- _players 1))))
    (`/Game/Multiplay/Blueprints/PlayerController_1.Kick` _asplayer_controller_1)))

(fn `GetCurrentPlayers`
  (returns (Players :type Integer))
  (bind _asgame_state_1 (cast `/Game/Multiplay/Blueprints/GameState_1` (`GameplayStatics.GetGameState`)))
  (for (_ _array_index) (`GameStateBase.PlayerArray` _asgame_state_1)
    _)
  (return (+ _array_index 1)))

(fn `UserConstructionScript`)