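; GameMode_1 is a multiplayer game mode that splits players across two teams and picks team-based spawn points.
; UpdateTeamID alternates LatestAllocatedTeamID between two values.
; ChoosePlayerStart reads TeamID from PlayerState_1 and returns a random PlayerStart whose tag matches that number.
; PlayerDied restarts the character's controller, but its binding to OnPlayerDied is unwired and never runs.
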(event `self.ReceiveBeginPlay`)

(event `PlayerDied` :!signature `self.OnPlayerDied`
  (params (Character :type "Character Object Reference"))
  (`self.RestartPlayer` (`Pawn.GetController` Character)))

(event `UpdateTeamID`
  (bind _latestallocatedteamid (`self.latestAllocatedTeamID`))
  (`/Engine/EditorBlueprintResources/StandardMacros.IncrementInt` _latestallocatedteamid
    (:`  `
      (set `self.latestAllocatedTeamID` (mod _latestallocatedteamid 2)))))

(fn `ChoosePlayerStart`
  (params (Player :type "Controller Object Reference"))
  (returns (ReturnValue :type "Actor Object Reference"))
  (bind _asplayer_state_1 (cast `/Game/Multiplay/Blueprints/PlayerState_1` (`Controller.PlayerState` Player)))
  (bind _outactors (`GameplayStatics.GetAllActorsOfClassWithTag` "/Script/Engine.PlayerStart" (`KismetStringLibrary.Conv_StringToName` (`KismetStringLibrary.Conv_IntToString` (`/Game/Multiplay/Blueprints/PlayerState_1.TeamID` _asplayer_state_1)))))
  (return (`KismetArrayLibrary.Array_Random` _outactors)))

(fn `UserConstructionScript`)